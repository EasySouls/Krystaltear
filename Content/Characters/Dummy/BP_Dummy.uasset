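; BP_Dummy is a target character that can be damaged or stealth-assassinated from behind by the player character BP_Ryonen.
; Damage goes through BPCPlayerStats, plays a random hit montage and launches the dummy along the player's forward vector, ragdolling it on death.
; An overlap radius toggles the assassination prompt, which turns with the healthbar widget toward the camera each tick.
; StealthBackAssassination plays the victim montage, delays ragdoll for the animation and returns the assassin's reference location and rotation.
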(event OnComponentBeginOverlap(AssassinationRadius)
  (params (OverlappedComponent :type Primitive%20Component%20Object%20Reference) (OtherActor :type Actor%20Object%20Reference) (OtherComp :type Primitive%20Component%20Object%20Reference) (OtherBodyIndex :type Integer) (bFromSweep :type Boolean) (SweepResult :type Hit%20Result%20Structure%20%28by%20ref%29))
  ;[1 1 1] Setting the visibility of the AssasinatePrompt widget
  (Utilities|Casting|CastToBP_Ryonen OtherActor)
  (Rendering|SetVisibility (Variables|Default|GetAssassinateWidget) true false))

(event OnComponentEndOverlap(AssassinationRadius)
  (params (OverlappedComponent :type Primitive%20Component%20Object%20Reference) (OtherActor :type Actor%20Object%20Reference) (OtherComp :type Primitive%20Component%20Object%20Reference) (OtherBodyIndex :type Integer))
  ;[1 1 1] Setting the visibility of the AssasinatePrompt widget
  (Utilities|Casting|CastToBP_Ryonen OtherActor)
  (Rendering|SetVisibility (Variables|Default|GetAssassinateWidget) false false))

(event Custom|Ragdoll
  ;[1 1 1] Ragdoll
  ; Delay is for the animation. If we enable physics while the animation is playing, it would cause it to stop
  (Utilities|FlowControl|Delay 2.5)
  (Physics|SetSimulatePhysics (Variables|Character|GetMesh) true))

(event Game|Damage|EventAnyDamage
  (params (Damage :type Float%20%28single-precision%29) (DamageType :type Damage%20Type%20Object%20Reference) (InstigatedBy :type Controller%20Object%20Reference) (DamageCauser :type Actor%20Object%20Reference))
  ;[1 1 1] On Damage
  (bind _isplayerdead (Default|TakeDamage (Variables|Default|GetBPC_PlayerStats) Damage))
  (Variables|Default|SetIsDead _isplayerdead)
  (Animation|PlayAnimMontage (Utilities|Array|Get(acopy) (Variables|Default|GetHitAnims) (Math|Random|RandomIntegerinRange 0 (- (Utilities|Array|Length (Variables|Default|GetHitAnims)) 1))) 1.0 "None")
  (bind _asbp_ryonen (Utilities|Casting|CastToBP_Ryonen (Game|GetPlayerCharacter 0)))
  (Character|LaunchCharacter (* (Math|Vector|GetForwardVector (Transformation|GetActorRotation _asbp_ryonen)) 7e+02) false false)
  (if (Variables|Default|GetIsDead)
    (Physics|SetSimulatePhysics (Variables|Character|GetMesh) true)
    (Rendering|SetVisibility (Variables|Default|GetHealthbarWidget) false false)))

(event EventBeginPlay
  ;[1 1 1] Save HealtbarWidget as a variable
  (bind _asbpw_dummy_healthbar (Utilities|Casting|CastToBPW_DummyHealthbar (UserInterface|GetWidget (Variables|Default|GetHealthbarWidget))))
  (Variables|Default|SetHealthbarUI _asbpw_dummy_healthbar))

(event EventTick
  (params (DeltaSeconds :type Float%20%28single-precision%29))
  ;[1 1 1] Tick
  ; Set the widgets towards the camera
  (Transformation|SetWorldRotation (Variables|Default|GetAssassinateWidget) (Math|Rotator|FindLookatRotation (Transformation|GetWorldLocation (Variables|Default|GetAssassinateWidget)) (Transformation|GetWorldLocation (Variables|/Script/Engine.PlayerCameraManager|GetTransformComponent (Game|GetPlayerCameraManager 0)))) false false))

(fn ConstructionScript)

(fn StealthBackAssassination
  (Animation|PlayAnimMontage "/Game/Characters/Ryonen/Animation/Assassinations/Paired_Knife_Stealth_KidneyAndNeck_Vic_Montage.Paired_Knife_Stealth_KidneyAndNeck_Vic_Montage" 1.0 "None")
  (CallFunction|Ragdoll)
  (Rendering|SetVisibility (Variables|Default|GetAssassinateWidget) false false)
  (return (Transformation|GetWorldLocation (Variables|Default|GetAssassinReference)) (Transformation|GetActorRotation)))