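; Attack component for BP_Ryonen that runs a four-step light attack combo of sword swings and a kick.
; The light attack input, gated by CanAttack, plays the montage for the current AttackIndex, with a short delay and DoOnce guard.
; Presses during an attack set SaveAttack, which SwordAttackCombo consumes to chain the next step.
; Without a buffered press, SwordAttackCombo calls StopCombo to reset the attack state and index.
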(event Custom|LightAttack
  (if (Variables|Default|GetIsAttacking)
    (Variables|Default|SetSaveAttack true)
    (else
      (Variables|Default|SetIsAttacking true)
      (switch int (Variables|Default|GetAttackIndex)
        (:0
          (CallFunction|SwordAttack1))
        (:1
          (CallFunction|SwordAttack2))
        (:2
          (CallFunction|SwordAttack3))
        (:3
          (CallFunction|SwordAttack4))))))

(event Custom|SwordAttackCombo
  (if (Variables|Default|GetSaveAttack)
    (Variables|Default|SetSaveAttack false)
    (switch int (Variables|Default|GetAttackIndex)
      (:0
        (CallFunction|SwordAttack1))
      (:1
        (CallFunction|SwordAttack2))
      (:2
        (CallFunction|SwordAttack3))
      (:3
        (CallFunction|SwordAttack4)))
    (else
      (CallFunction|StopCombo))))

(event Custom|StopCombo
  ;[1 1 1] Stop Combo Event
  ; Reset IsAttacking and AttackIndex for the combos
  (Variables|Default|SetIsAttacking false)
  (Variables|Default|SetAttackIndex 0))

(event Custom|SwordAttack4
  ;[1 1 1] Sword Attacks
  (Utilities|FlowControl|DoOnce false :!label _label
    (:Completed
      (Utilities|FlowControl|Delay 0.1)
      (Animation|Montage|PlayMontage (Variables|Default|GetCharacterMesh) "/Game/Characters/Ryonen/Animation/Attacks/Sword/Attack3_Montage.Attack3_Montage"
        (:then
          (Variables|Default|SetAttackIndex 0)
          (goto _label Reset))))))

(event Custom|SwordAttack1
  ;[1 1 1] Sword Attacks
  (Utilities|FlowControl|DoOnce false :!label _label
    (:Completed
      (Utilities|FlowControl|Delay 0.1)
      (Animation|Montage|PlayMontage (Variables|Default|GetCharacterMesh) "/Game/Characters/Ryonen/Animation/Attacks/Sword/Attack1_Montage.Attack1_Montage"
        (:then
          (Variables|Default|SetAttackIndex 1)
          (goto _label Reset))))))

(event Custom|SwordAttack2
  ;[1 1 1] Sword Attacks
  (Utilities|FlowControl|DoOnce false :!label _label
    (:Completed
      (Utilities|FlowControl|Delay 0.1)
      (Animation|Montage|PlayMontage (Variables|Default|GetCharacterMesh) "/Game/Characters/Ryonen/Animation/Attacks/Sword/Attack2_Montage.Attack2_Montage"
        (:then
          (Variables|Default|SetAttackIndex 2)
          (goto _label Reset))))))

(event Custom|SwordAttack3
  ;[1 1 1] Sword Attacks
  (Utilities|FlowControl|DoOnce false :!label _label
    (:Completed
      (Utilities|FlowControl|Delay 0.1)
      (Animation|Montage|PlayMontage (Variables|Default|GetCharacterMesh) "/Game/Characters/Ryonen/Animation/Attacks/Sword/Kick_Montage.Kick_Montage"
        (:then
          (Variables|Default|SetAttackIndex 3)
          (goto _label Reset))))))

(event Input|EnhancedActionEvents|EnhancedInputActionIA_LightAttack
  (params (ActionValue :type Boolean) (ElapsedSeconds :type Float%20%28double-precision%29) (TriggeredSeconds :type Float%20%28double-precision%29) (InputAction :type Input%20Action%20Object%20Reference :default "/Game/Blueprint/Input/Actions/IA_LightAttack.IA_LightAttack"))
  (:Started
    (if (Variables|Default|GetCanAttack)
      (CallFunction|LightAttack))))

(event EventBeginPlay
  ;[1 1 1] BeginPlay
  (Utilities|FlowControl|DelayUntilNextTick)
  (bind _asbp_ryonen (Utilities|Casting|CastToBP_Ryonen (Components|GetOwner)))
  (Variables|Default|SetCharacterMesh (Variables|/Script/Engine.Character|GetMesh _asbp_ryonen)))