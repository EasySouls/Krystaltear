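; BPC_InteractionComponent is a Blueprint component that tracks whether something can be interacted with and whether it is activated.
; Enable and disable events set the Interactable flag and broadcast OnToggleInteractibility.
; StartInteraction toggles Activated only while interactable and broadcasts OnInteract with the new state, so other objects can react.
; StopInteraction skips that check, broadcasting false before clearing Activated.
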(event Custom|DisableInteractivity
  ;[1 1 1] Enables interactivity and calls an event
  (bind _output_get (Variables|Default|SetInteractable false))
  (Default|CallOnToggleInteractibility _output_get))

(event Custom|EnableInteractivity
  ;[1 1 1] Enables interactivity and calls an event
  (bind _output_get (Variables|Default|SetInteractable true))
  (Default|CallOnToggleInteractibility _output_get))

(event Custom|StartInteraction
  ;[1 1 1] Event to start interaction, check if interaction is possible, save state, and call event so others can react to it
  (if (Variables|Default|GetInteractable)
    (bind _output_get (Variables|Default|SetActivated (not (Variables|Default|GetActivated))))
    (Default|CallOnInteract _output_get)))

(event Custom|StopInteraction
  ;[1 1 1] Event to stop interaction, call OnInteract and save state
  (Default|CallOnInteract false)
  (Variables|Default|SetActivated false))