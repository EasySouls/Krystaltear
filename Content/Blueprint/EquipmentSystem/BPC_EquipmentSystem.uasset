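; Equipment component for the BP_Ryonen character that handles weapon pickup and the inventory menu.
; Interact sphere-traces forward from the follow camera, adds a hit BP_Weapon's item data to the Inventory array and destroys the actor.
; The menu input toggles WB_Inventory and cursor, disabling movement on open; the nodes restoring game input and walking on close are unconnected.
; A debug key prints the inventory's row names.
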(event Input|EnhancedActionEvents|EnhancedInputActionIA_Interact
  (params (ActionValue :type Boolean) (ElapsedSeconds :type Float%20%28double-precision%29) (TriggeredSeconds :type Float%20%28double-precision%29) (InputAction :type Input%20Action%20Object%20Reference :default "/Game/Blueprint/Input/Actions/IA_Interact.IA_Interact"))
  (bind _followcamera (Variables|Default|GetFollowCamera))
  (bind _returnvalue (Transformation|GetWorldLocation _followcamera))
  ;[1 1 1] Picking up weapons
  (:Started
    (bind (_outhit _returnvalue_2) (Collision|SphereTraceForObjects _returnvalue (+ _returnvalue (* (Math|Vector|GetForwardVector (Transformation|GetWorldRotation _followcamera)) 5e+02)) 15.0 (Utilities|Array|MakeArray "ObjectTypeQuery2") false 0 "ForDuration" true "(R=1.000000,G=0.000000,B=0.000000,A=1.000000)" "(R=0.000000,G=1.000000,B=0.000000,A=1.000000)" 3.0))
    (if _returnvalue_2
      (bind _asbp_weapon (Utilities|Casting|CastToBP_Weapon (.HitActor (Collision|BreakHitResult _outhit))))
      (CallFunction|AddWeapon (Variables|/Game/Blueprint/EquipmentSystem/BP_Weapon.BP_Weapon_C|GetItemData _asbp_weapon))
      (Actor|DestroyActor _asbp_weapon))))

(event Input|EnhancedActionEvents|EnhancedInputActionIA_Menu
  (params (ActionValue :type Boolean) (ElapsedSeconds :type Float%20%28double-precision%29) (TriggeredSeconds :type Float%20%28double-precision%29) (InputAction :type Input%20Action%20Object%20Reference :default "/Game/Blueprint/Input/Actions/IA_Menu.IA_Menu"))
  (bind _returnvalue (Game|GetPlayerController 0))
  ;[1 1 1] Equipment menu widget
  (:Started
    (if (not (Variables|Default|GetIsMenuOpen))
      (Variables|Default|SetIsMenuOpen true)
      (bind _returnvalue_2 (UserInterface|CreateWidget "/Game/UI/WB_Inventory.WB_Inventory_C"))
      (bind _output_get (Variables|Default|SetEquipmentWidget _returnvalue_2))
      (UserInterface|Viewport|AddtoViewport _output_get 0)
      (Variables|/Script/Engine.PlayerController|SetbShowMouseCursor _returnvalue true)
      (Input|SetInputModeGameandUI _returnvalue (Variables|Default|GetEquipmentWidget) "DoNotLock" true false)
      (bind _asbp_ryonen (Utilities|Casting|CastToBP_Ryonen (Components|GetOwner)))
      (Pawn|Components|CharacterMovement|SetMovementMode (Variables|/Script/Engine.Character|GetCharacterMovement _asbp_ryonen) "MOVE_None" 0)
      (else
        (bind _equipmentwidget (Variables|Default|GetEquipmentWidget)
          (:then
            (Widget|RemovefromParent _equipmentwidget)
            (Variables|Default|SetIsMenuOpen false)
            (Variables|/Script/Engine.PlayerController|SetbShowMouseCursor _returnvalue false))
          (:else))))))

(event EventBeginPlay
  ;[1 1 1] Save the variables needed on BeginPlay
  (bind _asbp_ryonen (Utilities|Casting|CastToBP_Ryonen (Components|GetOwner)))
  (Variables|Default|SetFollowCamera (Variables|/Game/Characters/Ryonen/BP_Ryonen.BP_Ryonen_C|GetFollowCamera _asbp_ryonen)))

(event Input|KeyboardEvents|DebugKeyH
  (params (Key :type Key%20Structure :default "None") (ActionValue :type Input%20Action%20Value%20Structure))
  (:Pressed
    (for _array_element (Variables|Default|GetInventory)
      (Development|PrintText (Utilities|Text|ToText(Name) (.rowname (.item _array_element)))))))

(fn AddWeapon
  (params (NewWeapon :type S%20Slots%20Structure))
  (Utilities|Array|Add (Variables|Default|GetInventory) NewWeapon))