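; PC_InGame is the in-game player controller that sets up camera limits, input and the HUD, and handles pausing.
; On BeginPlay it clamps view pitch between looking down and level, switches to game-only input with a hidden cursor, and adds the BPW_HeadupDisplay widget to the viewport.
; IA_Pause toggles game pause, with F6 as an alternative key outside distribution builds.
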(event Input|EnhancedActionEvents|EnhancedInputActionIA_Pause
  (params (ActionValue :type Boolean) (ElapsedSeconds :type Float%20%28double-precision%29) (TriggeredSeconds :type Float%20%28double-precision%29) (InputAction :type Input%20Action%20Object%20Reference :default "/Game/Blueprint/Input/Actions/IA_Pause.IA_Pause"))
  ;[1 1 1] INPUT Pause Game
  (Game|SetGamePaused (not (Game|IsGamePaused))))

(event EventBeginPlay
  (bind _playercameramanager (Variables|Default|GetPlayerCameraManager))
  ;[1 1 1] BeginPlay
  (Utilities|FlowControl|Sequence
    (:then_0
      (Variables|/Script/Engine.PlayerCameraManager|SetViewPitchMin _playercameramanager -65.0)
      (Variables|/Script/Engine.PlayerCameraManager|SetViewPitchMax _playercameramanager 0.0))
    (:then_1
      (Input|SetInputModeGameOnly self false)
      (Variables|Default|SetbShowMouseCursor false))
    (:then_2
      (bind _returnvalue (UserInterface|CreateWidget "/Game/Blueprint/UI/BPW_HeadupDisplay.BPW_HeadupDisplay_C" self))
      (bind _output_get (Variables|Default|SetHeadupDisplay _returnvalue))
      (UserInterface|Viewport|AddtoViewport _output_get 0))))

(event Input|KeyboardEvents|F6
  (params (Key :type Key%20Structure :default "None"))
  ;[1 1 1] Only in development, since escape quits from the game
  (:Pressed
    (if (not (Class|KismetSystemLibrary|IsPackagedforDistribution))
      ;[1 1 1] INPUT Pause Game
      (Game|SetGamePaused (not (Game|IsGamePaused))))))

(fn ConstructionScript)