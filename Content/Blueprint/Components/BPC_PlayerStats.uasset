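; Stats component for the player (BP_Ryonen) or a dummy (BP_Dummy), tracking health, stamina, XP and level.
; On BeginPlay it waits a tick, then casts its owner to choose between the player HUD and the dummy's health bar.
; Damage and stamina depletion return true at zero or below, and each stat change pushes values straight to the widgets.
; Only TakeDamage supports the dummy; other updates assume the player, and each level-up raises the XP threshold.
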(event EventBeginPlay
  (bind _returnvalue (Components|GetOwner))
  ;[1 1 1] Waiting for the variables to be set
  (Utilities|FlowControl|DelayUntilNextTick)
  (bind _asbp_ryonen (Utilities|Casting|CastToBP_Ryonen _returnvalue)
    (:then
      ;[1 1 1] Casted to Player
      (Variables|Default|SetPlayerCharacterBP _asbp_ryonen)
      (bind _output_get (Variables|Default|SetIsPlayer true))
      (if _output_get
        (LevelandXP|UpdateXpBar)
        (Health|UpdateHealthBar (Health|GetHealthPercent) (Variables|Health|GetCurrentHealth))
        (Stamina|UpdateStaminaBar (/ (Variables|Stamina|GetCurrentStamina) (Variables|Stamina|GetMaxStamina)) (Variables|Stamina|GetCurrentStamina))))
    (:CastFailed
      ;[1 1 1] Cast to Dummy
      (bind _asbp_dummy (Utilities|Casting|CastToBP_Dummy _returnvalue))
      (Variables|Default|SetDummyBP _asbp_dummy)
      (Variables|Default|SetIsPlayer false)
      (Progress|SetPercent (Variables|/Game/UI/BPW_DummyHealthbar.BPW_DummyHealthbar_C|GetHealthBar (Variables|/Game/Characters/Dummy/BP_Dummy.BP_Dummy_C|GetHealthbarUI (Variables|Default|GetDummyBP))) (Health|GetHealthPercent)))))

(fn TakeDamage
  (params (DamageTaken :type Float%20%28double-precision%29))
  (if (not (<= (Variables|Health|GetCurrentHealth) 0))
    (bind _output_get (Variables|Health|SetCurrentHealth (- (Variables|Health|GetCurrentHealth) DamageTaken)))
    (if (Variables|Default|GetIsPlayer)
      (Health|UpdateHealthBar (Health|GetHealthPercent) (Variables|Health|GetCurrentHealth))
      (else
        (Progress|SetPercent (Variables|/Game/UI/BPW_DummyHealthbar.BPW_DummyHealthbar_C|GetHealthBar (Variables|/Game/Characters/Dummy/BP_Dummy.BP_Dummy_C|GetHealthbarUI (Variables|Default|GetDummyBP))) (Health|GetHealthPercent))))
    (if (<= (Variables|Health|GetCurrentHealth) 0)
      _
      (else
        (return false))))
  (return true))

(fn IncreaseMaxHealth
  (params (HealthGranted :type Float%20%28double-precision%29))
  (Variables|Health|SetMaxHealth (+ HealthGranted (Variables|Health|GetMaxHealth)))
  (Health|UpdateHealthBar (/ (Variables|Health|GetCurrentHealth) (Variables|Health|GetMaxHealth)) (Variables|Health|GetCurrentHealth)))

(fn DepleteStamina
  (params (StaminaDepleted :type Float%20%28double-precision%29))
  (if (not (<= (Variables|Stamina|GetCurrentStamina) 0.0))
    (bind _output_get (Variables|Stamina|SetCurrentStamina (- (Variables|Stamina|GetCurrentStamina) StaminaDepleted)))
    (Stamina|UpdateStaminaBar (/ _output_get (Variables|Stamina|GetMaxStamina)) (Variables|Stamina|GetCurrentStamina))
    (if (<= (Variables|Stamina|GetCurrentStamina) 0.0)
      _
      (else
        (return false))))
  (return true))

(fn IncreaseMaxStamina
  (params (StaminaGranted :type Float%20%28double-precision%29))
  (Variables|Stamina|SetMaxStamina (+ StaminaGranted (Variables|Stamina|GetMaxStamina)))
  (Stamina|UpdateStaminaBar (/ (Variables|Stamina|GetCurrentStamina) (Variables|Stamina|GetMaxStamina)) (Variables|Stamina|GetCurrentStamina)))

(fn IncreaseHealth
  (params (HealthIncrease :type Float%20%28double-precision%29))
  (Variables|Health|SetCurrentHealth (+ HealthIncrease (Variables|Health|GetCurrentHealth)))
  (if (> (Variables|Health|GetCurrentHealth) (Variables|Health|GetMaxHealth))
    (Variables|Health|SetCurrentHealth (Variables|Health|GetMaxHealth)))
  (Health|UpdateHealthBar (/ (Variables|Health|GetCurrentHealth) (Variables|Health|GetMaxHealth)) (Variables|Health|GetCurrentHealth)))

(fn IncreaseStamina
  (params (StaminaIncrease :type Float%20%28double-precision%29))
  (Variables|Stamina|SetCurrentStamina (+ StaminaIncrease (Variables|Stamina|GetCurrentStamina)))
  (if (> (Variables|Stamina|GetCurrentStamina) (Variables|Stamina|GetMaxStamina))
    (Variables|Stamina|SetCurrentStamina (Variables|Stamina|GetMaxStamina)))
  (Stamina|UpdateStaminaBar (/ (Variables|Stamina|GetCurrentStamina) (Variables|Stamina|GetMaxStamina)) (Variables|Stamina|GetCurrentStamina)))

(fn UpdateHealthBar
  (params (HealthPercent :type Float%20%28double-precision%29) (HealthText :type Float%20%28double-precision%29))
  (bind _playercharacterbp (Variables|Default|GetPlayerCharacterBP))
  (bind _hudwidget (Variables|/Game/Characters/Ryonen/BP_Ryonen.BP_Ryonen_C|GetHUDWidget _playercharacterbp))
  (Progress|SetPercent (Variables|/Game/UI/BPW_MainHUD.BPW_MainHUD_C|GetHealthBar _hudwidget) HealthPercent)
  (Rendering|Components|TextRender|SetText (Variables|/Game/UI/BPW_MainHUD.BPW_MainHUD_C|GetHealthText _hudwidget) (Utilities|Text|ToText(Float) HealthText "HalfToEven")))

(fn UpdateStaminaBar
  (params (StaminaPercent :type Float%20%28double-precision%29) (StaminaText :type Float%20%28double-precision%29))
  (bind _playercharacterbp (Variables|Default|GetPlayerCharacterBP))
  (bind _hudwidget (Variables|/Game/Characters/Ryonen/BP_Ryonen.BP_Ryonen_C|GetHUDWidget _playercharacterbp))
  (Progress|SetPercent (Variables|/Game/UI/BPW_MainHUD.BPW_MainHUD_C|GetStaminaBar _hudwidget) StaminaPercent)
  (Rendering|Components|TextRender|SetText (Variables|/Game/UI/BPW_MainHUD.BPW_MainHUD_C|GetStaminaText _hudwidget) (Utilities|Text|ToText(Float) StaminaText "HalfToEven")))

(fn IncreaseXP
  (params (AddedXp :type Integer))
  (Variables|XP|SetXP (+ AddedXp (Variables|XP|GetXP)))
  (if (>= (Variables|XP|GetXP) (Variables|XP|GetMaxXP))
    (LevelandXP|IncreaseLevel 1)
    (else
      (LevelandXP|UpdateXpBar))))

(fn IncreaseLevel
  (params (AddedLevel :type Integer))
  (Variables|XP|SetLevel (+ AddedLevel (Variables|XP|GetLevel)))
  (Variables|XP|SetXP (- (Variables|XP|GetXP) (Variables|XP|GetMaxXP)))
  (Variables|XP|SetMaxXP (+ (Variables|XP|GetMaxXP) 500))
  (LevelandXP|UpdateXpBar))

(fn UpdateXpBar
  (bind _playercharacterbp (Variables|Default|GetPlayerCharacterBP))
  (bind _hudwidget (Variables|/Game/Characters/Ryonen/BP_Ryonen.BP_Ryonen_C|GetHUDWidget _playercharacterbp))
  (Progress|SetPercent (Variables|/Game/UI/BPW_MainHUD.BPW_MainHUD_C|GetXPBar _hudwidget) (/ (Variables|XP|GetXP) (Math|Conversions|ToFloat(Integer) (Variables|XP|GetMaxXP))))
  (Rendering|Components|TextRender|SetText (Variables|/Game/UI/BPW_MainHUD.BPW_MainHUD_C|GetLevelText _hudwidget) (Utilities|Text|ToText(Integer) (Variables|XP|GetLevel)))
  (Rendering|Components|TextRender|SetText (Variables|/Game/UI/BPW_MainHUD.BPW_MainHUD_C|GetXPText _hudwidget) (Utilities|Text|FormatText "{CurrentXp} / {MaxXp}" (Variables|XP|GetXP) (Variables|XP|GetMaxXP))))

(fn GetHealthPercent
  (return (/ (Variables|Health|GetCurrentHealth) (Variables|Health|GetMaxHealth))))