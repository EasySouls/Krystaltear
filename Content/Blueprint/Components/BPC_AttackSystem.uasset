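; Attack component for BP_Ryonen that runs a four-step light-attack combo (sword, sword, kick, sword) and melee hit detection.
; Input during an attack is buffered in SaveAttack, and SwordAttackCombo either plays the next montage by AttackIndex or resets the combo.
; A looping timer sweeps along the blade, with a single sphere trace for other hits.
; Hits on "Damageable" actors apply damage, camera shake, sound and blood, with a cooldown on sword hits.
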(event Custom|LightAttack
  ;[1 1 1] Combo System
  (if (Variables|Default|GetIsAttacking)
    (Variables|Default|SetSaveAttack true)
    (else
      (Variables|Default|SetIsAttacking true)
      (switch int (Variables|Default|GetAttackIndex)
        (:0
          (CallFunction|SwordAttack1))
        (:1
          (CallFunction|SwordAttack2))
        (:2
          (CallFunction|SwordAttack3))
        (:3
          (CallFunction|SwordAttack4))))))

(event Custom|SwordAttackCombo
  ;[1 1 1] Combo System
  (if (Variables|Default|GetSaveAttack)
    (Variables|Default|SetSaveAttack false)
    (switch int (Variables|Default|GetAttackIndex)
      (:0
        (CallFunction|SwordAttack1))
      (:1
        (CallFunction|SwordAttack2))
      (:2
        (CallFunction|SwordAttack3))
      (:3
        (CallFunction|SwordAttack4)))
    (else
      (CallFunction|StopCombo))))

(event Custom|SphereTrace
  (bind _characterbp (Variables|Default|GetCharacterBP))
  (bind _spheretrace (Variables|/Game/Characters/Ryonen/BP_Ryonen.BP_Ryonen_C|GetSphereTrace _characterbp))
  (bind _returnvalue (Transformation|GetWorldLocation _spheretrace))
  ;[1 1 1] Generic Sphere Trace in front of the character
  (bind (_outhit _returnvalue_2) (Collision|SphereTraceByChannel _returnvalue _returnvalue 25.0 "TraceTypeQuery1" false 0 "None"))
  (if _returnvalue_2
    (if (Actor|ActorHasTag (.HitActor (Collision|BreakHitResult _outhit)) "Damageable")
      (Game|Damage|ApplyDamage (.HitActor (Collision|BreakHitResult _outhit)) 1e+01 0 0)
      (Camera|PlayWorldCameraShake "/Game/Blueprint/Components/CameraShake_OnEnemyHit.CameraShake_OnEnemyHit_C" (.Location (Collision|BreakHitResult _outhit)) 0.0 1e+03)
      (CallFunction|PlaySwordHitSounds)
      (Effects|SpawnEmitteratLocation "/Game/VFX_Pack/Particles/Blood/P_Blood_Splat_Cone.P_Blood_Splat_Cone" (.Location (Collision|BreakHitResult _outhit)) (Math|Rotator|MakeRotfromXY (.Normal (Collision|BreakHitResult _outhit)) (.Normal (Collision|BreakHitResult _outhit))) "1.000000,1.000000,1.000000" true "AutoRelease"))))

(event Custom|PlaySwordHitSounds
  ;[1 1 1] Sword hit sounds
  (Audio|PlaySoundatLocation "/Game/Audio/Combat/MS_SwordHit.MS_SwordHit" (Transformation|GetActorLocation (Variables|Default|GetCharacterBP)) "0, 0, 0" 1.0 1.0 0.0 0 0 0 0))

(event Custom|StopCombo
  ;[1 1 1] Combo System
  ;;[1 1 1] Stop Combo Event
  ;; Reset IsAttacking and AttackIndex for the combos
  (Variables|Default|SetIsAttacking false)
  (Variables|Default|SetAttackIndex 0))

(event Custom|SwordAttack4
  ;[1 1 1] Sword Attacks
  (Utilities|FlowControl|DoOnce false :!label _label
    (:Completed
      (Utilities|FlowControl|Delay 0.1)
      (Animation|Montage|PlayMontage (Variables|Default|GetCharacterMesh) "/Game/Characters/Ryonen/Animation/Attacks/Sword/Attack3_Montage.Attack3_Montage"
        (:then
          (Variables|Default|SetAttackIndex 0)
          (goto _label Reset))))))

(event Custom|SwordAttack1
  ;[1 1 1] Sword Attacks
  (Utilities|FlowControl|DoOnce false :!label _label
    (:Completed
      (Utilities|FlowControl|Delay 0.1)
      (Animation|Montage|PlayMontage (Variables|Default|GetCharacterMesh) "/Game/Characters/Ryonen/Animation/Attacks/Sword/Attack1_Montage.Attack1_Montage"
        (:then
          (Variables|Default|SetAttackIndex 1)
          (goto _label Reset))))))

(event Custom|Start%20SwordTrace
  ;[1 1 1] Sword Trace
  (bind _returnvalue (Utilities|Time|SetTimerbyEvent (delegate Custom|SwordTraceLoop) 0.001 true))
  (Variables|Default|SetSwordTraceTimer _returnvalue))

(event Custom|SwordAttack2
  ;[1 1 1] Sword Attacks
  (Utilities|FlowControl|DoOnce false :!label _label
    (:Completed
      (Utilities|FlowControl|Delay 0.1)
      (Animation|Montage|PlayMontage (Variables|Default|GetCharacterMesh) "/Game/Characters/Ryonen/Animation/Attacks/Sword/Attack2_Montage.Attack2_Montage"
        (:then
          (Variables|Default|SetAttackIndex 2)
          (goto _label Reset))))))

(event Custom|SwordTraceLoop
  (bind _characterbp (Variables|Default|GetCharacterBP))
  ;[1 1 1] Sword Trace
  (bind (_outhit _returnvalue) (Collision|SphereTraceByChannel (Transformation|GetWorldLocation (Variables|/Game/Characters/Ryonen/BP_Ryonen.BP_Ryonen_C|GetSwordTopPoint _characterbp)) (Transformation|GetWorldLocation (Variables|/Game/Characters/Ryonen/BP_Ryonen.BP_Ryonen_C|GetSwordBottomPoint _characterbp)) 12.0 "TraceTypeQuery1" false 0 "None"))
  (if _returnvalue
    (if (Actor|ActorHasTag (.HitActor (Collision|BreakHitResult _outhit)) "Damageable")
      (Utilities|FlowControl|DoOnce false :!label _label
        (:Completed
          (Game|Damage|ApplyDamage (.HitActor (Collision|BreakHitResult _outhit)) 25.0 0 0)
          (Camera|PlayWorldCameraShake "/Game/Blueprint/Components/CameraShake_OnEnemyHit.CameraShake_OnEnemyHit_C" (.Location (Collision|BreakHitResult _outhit)) 0.0 1e+03)
          (CallFunction|PlaySwordHitSounds)
          (Effects|SpawnEmitteratLocation "/Game/VFX_Pack/Particles/Blood/P_Blood_Splat_Cone.P_Blood_Splat_Cone" (.Location (Collision|BreakHitResult _outhit)) (Math|Rotator|MakeRotfromXY (.Normal (Collision|BreakHitResult _outhit)) (.Normal (Collision|BreakHitResult _outhit))) "1.000000,1.000000,1.000000" true "AutoRelease")
          (Utilities|FlowControl|Delay 0.5)
          (goto _label Reset))))))

(event Custom|SwordAttack3
  ;[1 1 1] Sword Attacks
  (Utilities|FlowControl|DoOnce false :!label _label
    (:Completed
      (Utilities|FlowControl|Delay 0.1)
      (Animation|Montage|PlayMontage (Variables|Default|GetCharacterMesh) "/Game/Characters/Ryonen/Animation/Attacks/Sword/Kick_Montage.Kick_Montage"
        (:then
          (Variables|Default|SetAttackIndex 3)
          (goto _label Reset))))))

(event Custom|StopSwordTrace
  ;[1 1 1] Sword Trace
  (Utilities|Time|ClearandInvalidateTimerbyHandle (Variables|Default|GetSwordTraceTimer)))

(event Input|EnhancedActionEvents|EnhancedInputActionIA_LightAttack
  (params (ActionValue :type Boolean) (ElapsedSeconds :type Float%20%28double-precision%29) (TriggeredSeconds :type Float%20%28double-precision%29) (InputAction :type Input%20Action%20Object%20Reference :default "/Game/Blueprint/Input/Actions/IA_LightAttack.IA_LightAttack"))
  ;[1 1 1] Combo System
  (:Started
    (if (Variables|Default|GetCanAttack)
      (CallFunction|LightAttack))))

(event EventBeginPlay
  ;[1 1 1] BeginPlay
  (Utilities|FlowControl|DelayUntilNextTick)
  (bind _asbp_ryonen (Utilities|Casting|CastToBP_Ryonen (Components|GetOwner)))
  (Variables|Default|SetCharacterBP _asbp_ryonen)
  (Variables|Default|SetCharacterMesh (Variables|/Script/Engine.Character|GetMesh _asbp_ryonen)))